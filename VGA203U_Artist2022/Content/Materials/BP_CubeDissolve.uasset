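; BP_CubeDissolve is an actor that feeds a cube's position and size to materials, apparently to drive a dissolve effect.
; It writes the Cube component's world location and world scale into the Pos1 and Bounds vector parameters of the PC_DATA parameter collection.
; The same write runs in the construction script and on every Tick, so the values update in the editor and track the cube at runtime.
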(event `self.ReceiveTick`
  (params (DeltaSeconds :type "Float (single-precision)"))
  (bind _cube (`self.Cube`))
  (`KismetMaterialLibrary.SetVectorParameterValue` "/Game/Materials/PC_DATA.PC_DATA" "Pos1" (`KismetMathLibrary.Conv_VectorToLinearColor` (`SceneComponent.K2_GetComponentLocation` _cube)))
  (`KismetMaterialLibrary.SetVectorParameterValue` "/Game/Materials/PC_DATA.PC_DATA" "Bounds" (`KismetMathLibrary.Conv_VectorToLinearColor` (`SceneComponent.K2_GetComponentScale` _cube))))

(fn `UserConstructionScript`
  (bind _cube (`self.Cube`))
  (`KismetMaterialLibrary.SetVectorParameterValue` "/Game/Materials/PC_DATA.PC_DATA" "Pos1" (`KismetMathLibrary.Conv_VectorToLinearColor` (`SceneComponent.K2_GetComponentLocation` _cube)))
  (`KismetMaterialLibrary.SetVectorParameterValue` "/Game/Materials/PC_DATA.PC_DATA" "Bounds" (`KismetMathLibrary.Conv_VectorToLinearColor` (`SceneComponent.K2_GetComponentScale` _cube))))